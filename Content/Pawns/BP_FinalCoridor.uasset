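; BP_FinalCoridor is a corridor-end trigger that can loop the player back toward their starting position.
; On BeginPlay it records the first MainCharacter's location.
; Any overlap calls IncreaseNumberOfIterations on BP_CounterOfPapers, before the character cast; a true result permits the teleport.
; The teleport shifts MainCharacter by the XY delta from the Cube to that start, preserving height and offset relative to the Cube.
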(event EventBeginPlay
  (bind _outactors (Actor|GetAllActorsOfClass "/Game/Pawns/MainCharacter.MainCharacter_C"))
  (Variables|Default|SetStartPosition (Transformation|GetWorldLocation (Variables|/Game/Pawns/MainCharacter.MainCharacter_C|GetDefaultSceneRoot (Utilities|Array|Get(acopy) _outactors)))))

(event Collision|EventActorBeginOverlap
  (params (OtherActor :type Actor%20Object%20Reference))
  (bind _self self)
  (bind _startposition (Variables|Default|GetStartPosition))
  (bind _cube (Variables|Default|GetCube _self))
  (bind _returnvalue (Transformation|GetWorldLocation _cube))
  (bind _returnvalue_2 (- (Math|Vector|MakeVector (.x _startposition) (.y _startposition) 0.0) (Math|Vector|MakeVector (.x _returnvalue) (.y _returnvalue) 0.0)))
  (bind _outactors (Actor|GetAllActorsOfClass "/Game/Pawns/BP_CounterOfPapers.BP_CounterOfPapers_C"))
  (bind _less (Default|IncreaseNumberOfIterations (Utilities|Array|Get(acopy) _outactors)))
  (if _less
    (bind _asmain_character (Utilities|Casting|CastToMainCharacter OtherActor))
    (Transformation|AddActorWorldOffset _asmain_character (Math|Vector|MakeVector (.x _returnvalue_2) (.y _returnvalue_2) 0.0) false true)))

(fn ConstructionScript)